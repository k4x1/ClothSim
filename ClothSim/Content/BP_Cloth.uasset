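; BP_Cloth is a cloth actor with a wind indicator arrow and a release action.
; Each tick it rotates the arrow root to the wind rotation and lengthens the arrow with the wind vector's magnitude through a lerp.
; A DropCloth event calls ReleaseCloth, and the construction script is empty.
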(event `self.ReceiveTick`
  (params (DeltaSeconds :type "Float (single-precision)"))
  (`SceneComponent.K2_SetWorldRotation` (`self.AroowRoot`) (`self.WindRotation`) false false)
  (set `ArrowComponent.ArrowLength` (`KismetMathLibrary.Lerp` 30.0 150.0 (/ (- (`KismetMathLibrary.VSize` (`self.WindVector`)) 500.0) 1500.0)) (`self.Arrow`)))

(event `Drop Cloth`
  (`self.ReleaseCloth`))

(fn `UserConstructionScript`)